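; BP_Topf is a cooking pot that reacts once both milk (Milch) and cocoa (Kakao) are flagged in the GI_Basic game instance.
; Its Moveable event checks those flags, then rescales the Cylinder component into a thin disc, likely the liquid.
; After timed delays it restarts a Niagara effect with a boiling-water sound, then plays a Level Sequence if one is valid.
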(event `/Game/Blueprints/Interface/BPI_Moveable.Moveable`
  (bind _gi_basic (`self.GI Basic`))
  (bind _niagara (`self.Niagara`))
  (bind _asgi_basic (cast `/Game/Blueprints/GI_Basic` (`GameplayStatics.GetGameInstance`)))
  (set `self.GI Basic` _asgi_basic)
  (if (and (`/Game/Blueprints/GI_Basic.Milch` _gi_basic) (`/Game/Blueprints/GI_Basic.Kakao` _gi_basic))
    (`SceneComponent.SetWorldScale3D` (`self.Cylinder`) (0.5 0.5 0.02))
    (`KismetSystemLibrary.Delay` 2.0)
    (`ActorComponent.SetAutoActivate` _niagara true)
    (`NiagaraComponent.ResetSystem` _niagara)
    (`GameplayStatics.PlaySound2D` "/Game/Audio/Sounds/MS_BoilingWater.MS_BoilingWater" 1.0 1.0 0.0 null null)
    (`KismetSystemLibrary.Delay` 4.0)
    (bind _levelsequence (`self.LevelSequence`)
      (:`then`
        (`MovieSceneSequencePlayer.Play` (`LevelSequenceActor.SequencePlayer` _levelsequence)))
      (:`else`))))

(fn `UserConstructionScript`)