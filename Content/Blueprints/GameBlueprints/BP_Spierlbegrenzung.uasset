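; Play-boundary actor that lights up with a fire crackle and removes its two Box components when collected.
; Collect caches GM_Basic, restarts the Niagara effect, reveals the point light and destroys Box and Box1.
; It then plays the crackle sound in 2D and has the game mode set up the cozy music.
; Overlap and Tick are empty, and nothing in this graph calls Collect.
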(event `/Game/Blueprints/Interface/BPI_Collectable.Collect`
  (bind _niagara (`self.Niagara`))
  (bind _asgm_basic (cast `/Game/Blueprints/GM_Basic` (`GameplayStatics.GetGameMode`)))
  (set `self.GM Basic` _asgm_basic)
  (`ActorComponent.SetAutoActivate` _niagara true)
  (`NiagaraComponent.ResetSystem` _niagara)
  (`SceneComponent.SetHiddenInGame` (`self.PointLight`) false false)
  (`ActorComponent.K2_DestroyComponent` (`self.Box`))
  (`ActorComponent.K2_DestroyComponent` (`self.Box1`))
  (`GameplayStatics.PlaySound2D` "/Game/Audio/Sounds/MS_FireCrackle.MS_FireCrackle" 1.0 1.0 0.0 null null)
  (`/Game/Blueprints/GM_Basic.Setup Cozy Musik` (`self.GM Basic`)))

(fn `UserConstructionScript`)