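; BP_Kakao is a collectible cocoa item for a quest.
; Its Collect event sets the Kakao flag on the GI_Basic game instance.
; If Quest3 is active, it destroys itself, first advancing the quest to stage 6 when Milch is also held.
; Without Quest3 the flag is still set but the actor stays in the world.
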(event `/Game/Blueprints/Interface/BPI_Collectable.Collect`
  (bind __gi_basic (`self. GI Basic`))
  (bind _asgi_basic (cast `/Game/Blueprints/GI_Basic` (`GameplayStatics.GetGameInstance`)))
  (bind _output_get (set `self. GI Basic` _asgi_basic))
  (set `/Game/Blueprints/GI_Basic.Kakao` true _output_get)
  (if (`/Game/Blueprints/GI_Basic.Quest3` _output_get)
    (if (and (`/Game/Blueprints/GI_Basic.Kakao` __gi_basic) (`/Game/Blueprints/GI_Basic.Milch` __gi_basic))
      (`/Game/Blueprints/GI_Basic.Update Quest Stage` (`self. GI Basic`) 6)
      (`self.K2_DestroyActor`)
      (else
        (`self.K2_DestroyActor`)))))

(fn `UserConstructionScript`)