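; Possessable object that the player takes control of through Interact and leaves with an exit input, which hands possession back to BP_Player.
; While possessed, left click traces under the cursor for WorldDynamic objects and stores moveable or collectable hits as the current interactable.
; Left click also sends collect and move interface messages to that interactable.
; Collectable targets are cleared after a short delay, and exiting clears any target.
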(event `/Game/Blueprints/Interface/BPI_Interactable.Interact`
  (`Controller.Possess` (`GameplayStatics.GetPlayerController` 0) self))

(event `EnhancedInput|/Game/Inputs/IA_ExitPossessed`
  (params (ActionValue :type Boolean) (ElapsedSeconds :type "Float (double-precision)") (TriggeredSeconds :type "Float (double-precision)") (InputAction :type "InputAction Object Reference" :default "/Game/Inputs/IA_ExitPossessed.IA_ExitPossessed"))
  (:`Started`
    (`self.ExitPossessable`)))

(event `ExitPossessable`
  (bind _returnvalue (`GameplayStatics.GetActorOfClass` "/Game/Blueprints/BP_Player.BP_Player_C"))
  (`Controller.Possess` (`GameplayStatics.GetPlayerController` 0) _returnvalue)
  (set `self.Current Interactable` null))

(event `EnhancedInput|/Game/Inputs/IA_LeftMouseButton`
  (params (ActionValue :type Boolean) (ElapsedSeconds :type "Float (double-precision)") (TriggeredSeconds :type "Float (double-precision)") (InputAction :type "InputAction Object Reference" :default "/Game/Inputs/IA_LeftMouseButton.IA_LeftMouseButton"))
  ;[1 0.1529 0.1529] Mouse Click | Posses Interactable Objects
  (:`Started`
    (bind _asplayer_controller (cast `PlayerController` (`self.GetController`)))
    (bind (_hitresult _returnvalue) (`PlayerController.GetHitResultUnderCursorForObjects` _asplayer_controller (`|MakeArray` "ObjectTypeQuery2" :!type "EObjectTypeQuery Enum") true))
    (if _returnvalue
      (`|ExecutionSequence`
        (:`then_0`
          (bind (_bblockinghit _binitialoverlap _time _distance _location _impactpoint _normal _impactnormal _physmat _hitactor) (`GameplayStatics.BreakHitResult` _hitresult))
          (if (`KismetSystemLibrary.DoesImplementInterface` _hitactor "/Game/Blueprints/Interface/BPI_Moveable.BPI_Moveable_C")
            (set `self.Current Interactable` _hitactor)))
        (:`then_1`
          (if (`KismetSystemLibrary.DoesImplementInterface` _hitactor "/Game/Blueprints/Interface/BPI_Collectable.BPI_Collectable_C")
            (set `self.Current Interactable` _hitactor)
            (`self.ClearCurrentInteractble`)))))))

(event `EnhancedInput|/Game/Inputs/IA_LeftMouseButton`
  (params (ActionValue :type Boolean) (ElapsedSeconds :type "Float (double-precision)") (TriggeredSeconds :type "Float (double-precision)") (InputAction :type "InputAction Object Reference" :default "/Game/Inputs/IA_LeftMouseButton.IA_LeftMouseButton"))
  (bind _current_interactable (`self.Current Interactable`))
  ;[1 0.1529 0.1529] Mouse Click | Posses Interactable Objects
  ;;[1 1 1] Trigger BP-Interface Event on Objects
  (:`Started`
    (`|ExecutionSequence`
      (:`then_0`
        (message `/Game/Blueprints/Interface/BPI_Collectable.Collect` _current_interactable))
      (:`then_1`
        (message `/Game/Blueprints/Interface/BPI_Moveable.Moveable` _current_interactable)))))

(event `ClearCurrentInteractble`
  ;[1 0.1529 0.1529] Mouse Click | Posses Interactable Objects
  ;;[1 0.1529 0.1529] Clear Current Moveable Interactable after Time | :3
  (`KismetSystemLibrary.Delay` 0.2)
  (set `self.Current Interactable` null))

(fn `UserConstructionScript`)