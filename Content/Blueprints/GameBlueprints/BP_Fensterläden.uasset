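; Window shutter actor (Fensterläden) that the player can set in place as a quest step once they have a nail and a hammer.
; Its Moveable event checks the Nail and Hammer flags on the GI_Basic game instance.
; When both are set, it snaps the actor to a hardcoded relative position and tilt, then advances the quest stage and updates the dialogue through the game instance.
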(event `/Game/Blueprints/Interface/BPI_Moveable.Moveable`
  (bind _gi_basic (`self.GI Basic`))
  (bind _asgi_basic (cast `/Game/Blueprints/GI_Basic` (`GameplayStatics.GetGameInstance`)))
  (bind _output_get (set `self.GI Basic` _asgi_basic))
  (if (and (`/Game/Blueprints/GI_Basic.Nail` _output_get) (`/Game/Blueprints/GI_Basic.Hammer` _output_get))
    (`self.K2_SetActorRelativeRotation` (`KismetMathLibrary.MakeRotator` -10.0))
    (`self.K2_SetActorRelativeLocation` (50.0 390.0 100.0))
    (`/Game/Blueprints/GI_Basic.Update Quest Stage` _gi_basic 2)
    (`/Game/Blueprints/GI_Basic.Update Dialogue` _gi_basic)))

(fn `UserConstructionScript`)