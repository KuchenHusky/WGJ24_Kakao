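; BP_Nail is a collectible nail pickup that feeds progress into a quest.
; Its Collect event sets the Nail flag on the GI_Basic game instance.
; While Quest2 is active it advances the quest stage if the Hammer is also held, then destroys itself.
; When Quest2 is inactive, the flag is still set but the actor stays in the world.
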(event `/Game/Blueprints/Interface/BPI_Collectable.Collect`
  (bind __gi_basic (`self. GI Basic`))
  (bind __gi_basic_2 (`self. GI Basic`))
  (bind _asgi_basic (cast `/Game/Blueprints/GI_Basic` (`GameplayStatics.GetGameInstance`)))
  (set `self. GI Basic` _asgi_basic)
  (set `/Game/Blueprints/GI_Basic.Nail` true __gi_basic)
  (if (`/Game/Blueprints/GI_Basic.Quest2` __gi_basic)
    (if (and (`/Game/Blueprints/GI_Basic.Hammer` __gi_basic_2) (`/Game/Blueprints/GI_Basic.Nail` __gi_basic_2))
      (`/Game/Blueprints/GI_Basic.Update Quest Stage` (`self. GI Basic`) 4)
      (`self.K2_DestroyActor`)
      (else
        (`self.K2_DestroyActor`)))))

(fn `UserConstructionScript`)