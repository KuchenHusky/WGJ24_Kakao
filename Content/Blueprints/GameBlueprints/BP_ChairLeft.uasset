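; BP_ChairLeft is a chair that the player can set upright as part of the first quest.
; Its Moveable event, active while Quest1 is set in GI_Basic, increments the shared chair count and zeroes the root's roll and pitch while keeping yaw.
; When the chair and spider web counts both reach their thresholds, it advances the quest stage, updates dialogue and ends Quest1 through the game instance.
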(event `/Game/Blueprints/Interface/BPI_Moveable.Moveable`
  (bind _gi_basic (`self.GI Basic`))
  (bind _defaultsceneroot (`self.DefaultSceneRoot`))
  (bind _gi_basic_2 (`self.GI Basic`))
  (bind _gi_basic_3 (`self.GI Basic`))
  (bind (_returnvalue_roll _returnvalue_pitch _returnvalue_yaw) (`KismetMathLibrary.BreakRotator` (`SceneComponent.GetSocketRotation` _defaultsceneroot "None")))
  (bind _asgi_basic (cast `/Game/Blueprints/GI_Basic` (`GameplayStatics.GetGameInstance`)))
  (bind _output_get (set `self.GI Basic` _asgi_basic))
  (if (`/Game/Blueprints/GI_Basic.Quest1` _output_get)
    (bind _result (`/Engine/EditorBlueprintResources/StandardMacros.IncrementInt` (`/Game/Blueprints/GI_Basic.ChairCount` _gi_basic))
      (:`  `
        (set `/Game/Blueprints/GI_Basic.ChairCount` _result _gi_basic)
        (`SceneComponent.K2_SetRelativeRotation` _defaultsceneroot (`KismetMathLibrary.MakeRotator` 0.0 0.0 _returnvalue_yaw) false false)
        (if (and (>= (`/Game/Blueprints/GI_Basic.ChairCount` _gi_basic_2) 2) (>= (`/Game/Blueprints/GI_Basic.SpiderWebCount` _gi_basic_2) 3))
          (`/Game/Blueprints/GI_Basic.Update Quest Stage` _gi_basic_3 2)
          (`/Game/Blueprints/GI_Basic.Update Dialogue` _gi_basic_3)
          (`/Game/Blueprints/GI_Basic.End Quest1` _gi_basic_3))))))

(fn `UserConstructionScript`)