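; BP_Hammer is a collectible hammer item that feeds into the second quest.
; Its Collect event gets GI_Basic from the game instance and does nothing unless the Quest2 flag is set.
; When it is, the event sets the Hammer flag, advances the quest stage if the Nail flag is also set, and destroys the actor either way.
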(event `/Game/Blueprints/Interface/BPI_Collectable.Collect`
  (bind _gi_basic (`self.GI Basic`))
  (bind _gi_basic_2 (`self.GI Basic`))
  (bind _asgi_basic (cast `/Game/Blueprints/GI_Basic` (`GameplayStatics.GetGameInstance`)))
  (bind _output_get (set `self.GI Basic` _asgi_basic))
  (if (`/Game/Blueprints/GI_Basic.Quest2` _output_get)
    (if (`/Game/Blueprints/GI_Basic.Nail` _output_get)
      (set `/Game/Blueprints/GI_Basic.Hammer` true _gi_basic)
      (if (and (`/Game/Blueprints/GI_Basic.Hammer` _gi_basic_2) (`/Game/Blueprints/GI_Basic.Nail` _gi_basic_2))
        (`/Game/Blueprints/GI_Basic.Update Quest Stage` (`self.GI Basic`) 4)
        (`self.K2_DestroyActor`)
        (else
          (`self.K2_DestroyActor` :!label _label)))
      (else
        (set `/Game/Blueprints/GI_Basic.Hammer` true _gi_basic)
        (goto _label)))))

(fn `UserConstructionScript`)