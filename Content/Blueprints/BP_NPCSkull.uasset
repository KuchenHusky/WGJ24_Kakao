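; Possessable NPC skull that the player controller takes over on interaction, opening dialog through GM_Basic.
; The exit input hands control back to BP_Player, clears the current interactable and calls OpenDialogUI again.
; Left click sends collect and moveable messages to CurrentInteractable, but the cursor trace that would assign it via the collectable and moveable interfaces is disconnected.
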(event `self.ReceiveBeginPlay`
  (`self.SetupGameMode`))

(event `SetupGameMode`
  (bind _asgm_basic (cast `/Game/Blueprints/GM_Basic` (`GameplayStatics.GetGameMode`)))
  (set `self.GM Basic` _asgm_basic))

(event `/Game/Blueprints/Interface/BPI_Interactable.Interact`
  (`Controller.Possess` (`GameplayStatics.GetPlayerController` 0) self)
  (`KismetSystemLibrary.PrintString` "I AM POSSED")
  (`/Game/Blueprints/GM_Basic.OpenDialogUI` (`self.GM Basic`)))

(event `EnhancedInput|/Game/Inputs/IA_ExitPossessed`
  (params (ActionValue :type Boolean) (ElapsedSeconds :type "Float (double-precision)") (TriggeredSeconds :type "Float (double-precision)") (InputAction :type "InputAction Object Reference" :default "/Game/Inputs/IA_ExitPossessed.IA_ExitPossessed"))
  (:`Started`
    (`self.ExitPossessable`)))

(event `ExitPossessable`
  (bind _returnvalue (`GameplayStatics.GetActorOfClass` "/Game/Blueprints/BP_Player.BP_Player_C"))
  (`Controller.Possess` (`GameplayStatics.GetPlayerController` 0) _returnvalue)
  (set `self.Current Interactable` null)
  (`/Game/Blueprints/GM_Basic.OpenDialogUI` (`self.GM Basic`)))

(event `EnhancedInput|/Game/Inputs/IA_LeftMouseButton`
  (params (ActionValue :type Boolean) (ElapsedSeconds :type "Float (double-precision)") (TriggeredSeconds :type "Float (double-precision)") (InputAction :type "InputAction Object Reference" :default "/Game/Inputs/IA_LeftMouseButton.IA_LeftMouseButton"))
  ;[1 0.1529 0.1529] Mouse Click | Posses Interactable Objects
)

(event `EnhancedInput|/Game/Inputs/IA_LeftMouseButton`
  (params (ActionValue :type Boolean) (ElapsedSeconds :type "Float (double-precision)") (TriggeredSeconds :type "Float (double-precision)") (InputAction :type "InputAction Object Reference" :default "/Game/Inputs/IA_LeftMouseButton.IA_LeftMouseButton"))
  (bind _current_interactable (`self.Current Interactable`))
  ;[1 0.1529 0.1529] Mouse Click | Posses Interactable Objects
  ;;[1 1 1] Trigger Interact Event on Interactable Objects
  (:`Started`
    (`|ExecutionSequence`
      (:`then_0`
        (message `/Game/Blueprints/Interface/BPI_Collectable.Collect` _current_interactable))
      (:`then_1`
        (message `/Game/Blueprints/Interface/BPI_Moveable.Moveable` _current_interactable)))))

(event `ClearCurrentInteractble`
  ;[1 0.1529 0.1529] Mouse Click | Posses Interactable Objects
  ;;[1 0.1529 0.1529] Clear Current Moveable Interactable after Time | :3
  (`KismetSystemLibrary.Delay` 0.2)
  (set `self.Current Interactable` null))

(fn `UserConstructionScript`)