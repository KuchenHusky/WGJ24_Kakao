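; GM_Basic is a basic game mode that owns the in-game UI and handles pausing.
; On begin play it creates the WBP_GameUI root widget and pushes the gameplay UI onto its gameplay widget stack, then enables the cursor with game-and-UI input.
; PauseGame pushes the pause menu onto a separate pause stack, pauses the game and switches to UI-only input, while UnPauseGame clears that stack and restores game-and-UI input.
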(event `self.ReceiveBeginPlay`
  (bind _returnvalue (`GameplayStatics.GetPlayerController` 0))
  (`self.Setup UI`)
  (set `PlayerController.bShowMouseCursor` true _returnvalue)
  (`WidgetBlueprintLibrary.SetInputMode_GameAndUIEx` _returnvalue null))

(event `self.ReceiveTick`
  (params (DeltaSeconds :type "Float (single-precision)")))

(event `Setup UI`
  ;[1 1 1] In Game UI
  (bind _returnvalue (`|CreateWidget` "/Game/BlueprintsUI/WBP_GameUI.WBP_GameUI_C"))
  (bind _output_get (set `self.GameUI` _returnvalue))
  (`UserWidget.AddToViewport` _output_get 0)
  (`CommonActivatableWidgetContainerBase.BP_AddWidget` (`/Game/BlueprintsUI/WBP_GameUI.GameplayStack` _output_get) "/Game/BlueprintsUI/WBP_GameplayUI.WBP_GameplayUI_C"))

(event `Pause Game`
  (bind _returnvalue (`GameplayStatics.GetPlayerController` 0))
  ;[1 1 1] PauseGame
  (`CommonActivatableWidgetContainerBase.BP_AddWidget` (`/Game/BlueprintsUI/WBP_GameUI.PauseStack` (`self.GameUI`)) "/Game/BlueprintsUI/WBP_PauseMenuBase.WBP_PauseMenuBase_C")
  (`GameplayStatics.SetGamePaused` true)
  (set `PlayerController.bShowMouseCursor` true _returnvalue)
  (`WidgetBlueprintLibrary.SetInputMode_UIOnlyEx` _returnvalue null))

(event `UnPause Game`
  (bind _returnvalue (`GameplayStatics.GetPlayerController` 0))
  ;[1 1 1] UnpauseGame
  (`CommonActivatableWidgetContainerBase.ClearWidgets` (`/Game/BlueprintsUI/WBP_GameUI.PauseStack` (`self.GameUI`)))
  (`GameplayStatics.SetGamePaused` false)
  (set `PlayerController.bShowMouseCursor` true _returnvalue)
  (`WidgetBlueprintLibrary.SetInputMode_GameAndUIEx` _returnvalue null))

(fn `UserConstructionScript`)