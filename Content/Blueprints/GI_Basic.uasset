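; Game instance that holds quest progress: quest stage, spider web and chair counts, and the first quest's completion flag.
; Stage updates check completion against both count thresholds, then push the stage to the active gameplay widget through GMBasic.
; Dialogue updates advance DialogUI, opening it first only while either count is short.
; Init is empty; game mode caching and persistent music code are disconnected.
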(event `self.ReceiveInit`)

(event `Update Quest Stage`
  (params (QuestIndex :type Integer))
  (`self.End Quest1`)
  (bind _output_get (set `self.QuestStage` QuestIndex))
  (bind _aswbp_gameplay_ui (cast `/Game/BlueprintsUI/WBP_GameplayUI` (`CommonActivatableWidgetContainerBase.GetActiveWidget` (`/Game/BlueprintsUI/WBP_GameUI.GameplayStack` (`/Game/Blueprints/GM_Basic.GameUI` (`self.GM Basic`))))))
  (`/Game/BlueprintsUI/WBP_GameplayUI.Update Quest Stage` _aswbp_gameplay_ui _output_get))

(event `Update Dialogue`
  (if (and (>= (`self.SpiderWebCount`) 3) (>= (`self.ChairCount`) 2))
    (`/Game/BlueprintsUI/WBP_Dialogbox.Update Dialogue` (`self.DialogUI`))
    (`KismetSystemLibrary.PrintString` "dialog" true true (struct :`G` 0.66 :`B` 1.0 :`A` 1.0) 60.0)
    (else
      (`/Game/Blueprints/GM_Basic.OpenDialogUI` (`self.GM Basic`))
      (`/Game/BlueprintsUI/WBP_Dialogbox.Update Dialogue` (`self.DialogUI`))
      (`self.End Quest1`))))

(event `End Quest1`
  (if (and (>= (`self.SpiderWebCount`) 3) (>= (`self.ChairCount`) 2))
    (set `self.Quest1End` true)))